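; BP_ItemInstance is a runtime inventory item that pairs a DA_ItemDefinition with its own count and durability.
; Init stores the definition, starts durability at its maximum and clamps the count between one and the max stack.
; Use delegates to a BP_ItemBehavior object, lazily constructed and cached by EnsureBehavior, always from that same class.
; Throw is empty, and CanBeThrown and the count, name and icon getters return placeholder values.
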(event EventUse
  (params (User :type BP%20Combat%20Character%20Base%20Object%20Reference))
  (bind _behavior (CallFunction|EnsureBehavior))
  (Default|ExecuteUse _behavior User))

(event EventThrow
  (params (User :type Character%20Object%20Reference)))

(fn Init
  (params (Def :type DA%20Collectible%20Definition%20Object%20Reference) (InCount :type Integer))
  ;[0.15 0.03895 0.1076 0.5] Init Funciton
  (bind _output_get (Variables|Default|SetDefinition Def))
  (bind _asda_item_definition (Utilities|Casting|CastToDA_ItemDefinition _output_get))
  (Variables|Default|SetDurability (Variables|/Game/Blueprins/Inventory/DA_ItemDefinition.DA_ItemDefinition_C|GetDurabilityMax _asda_item_definition))
  (Variables|Default|SetCount (Math|Integer|Clamp(Integer) InCount 1 (Variables|/Game/Blueprins/Inventory/DA_CollectibleDefinition.DA_CollectibleDefinition_C|GetMaxStack _output_get))))

(fn EnsureBehavior
  ;[0.15 0.02917 0.1332 0.5] Init Behaviour
  (if (Utilities|IsValid (Variables|Default|GetBehavior))
    (return (Variables|Default|GetBehavior))
    (else
      (bind _returnvalue (Game|ConstructObjectfromClass "/Game/Blueprins/Inventory/BP_ItemBehavior.BP_ItemBehavior_C"))
      (bind _output_get (Variables|Default|SetBehavior _returnvalue))
      (return _output_get))))

(fn CanbeThrown
  (return false))

(fn GetCount
  (return 0))

(fn GetDisplayName
  (return ""))

(fn GetIcon
  (return ""))