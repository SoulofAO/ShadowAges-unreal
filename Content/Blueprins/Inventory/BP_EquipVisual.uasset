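; BP_EquipVisual is an actor that displays the mesh of an inventory item, taken from its ItemDefinition.
; The construction script uses the definition's skeletal mesh when it is valid, otherwise its static mesh.
; It assigns that mesh to the matching component, shows it and hides the other, propagating visibility to children.
; The event graph holds only disabled placeholder events, so there is no runtime logic.
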(event EventBeginPlay)

(event Collision|EventActorBeginOverlap
  (params (OtherActor :type Actor%20Object%20Reference)))

(event EventTick
  (params (DeltaSeconds :type Float%20%28single-precision%29)))

(fn ConstructionScript
  (bind _skeletalmeshcomp (Variables|Default|GetSkeletalMeshComp))
  (bind _itemdefinition (Variables|Default|GetItemDefinition))
  (bind _staticmeshcomp (Variables|Default|GetStaticMeshComp))
  ;[0.5781 0 0.02089 0.5] Begin Play
  (if (Utilities|IsValid (Variables|/Game/Blueprins/Inventory/BP_ItemDefinition.BP_ItemDefinition_C|GetSkeletalMesh (Variables|Default|GetItemDefinition)))
    (Components|SkeletalMesh|SetSkeletalMeshAsset _skeletalmeshcomp (Variables|/Game/Blueprins/Inventory/BP_ItemDefinition.BP_ItemDefinition_C|GetSkeletalMesh _itemdefinition))
    (Rendering|SetVisibility _skeletalmeshcomp true true)
    (Rendering|SetVisibility (Variables|Default|GetStaticMeshComp) false true)
    (else
      (Components|StaticMesh|SetStaticMesh _staticmeshcomp (Variables|/Game/Blueprins/Inventory/BP_ItemDefinition.BP_ItemDefinition_C|GetStaticMesh _itemdefinition))
      (Rendering|SetVisibility _staticmeshcomp true true)
      (Rendering|SetVisibility (Variables|Default|GetSkeletalMeshComp) false true))))