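; Inventory actor for player 0's character, storing item instances with stack-aware adding, removal and change dispatchers.
; The active index wraps through the items plus an empty-hand slot.
; Equipping either spawns the definition's actor on a mesh socket, offset by its own inverted socket transform, or constructs a behavior object.
; Use and throw forward to these through IBP_InventoryItem, and throwing also launches a BP_WorldPickup.
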(event EventBeginPlay
  (Variables|Default|SetOwnerCharacter (Game|GetPlayerCharacter 0)))

(event Collision|EventActorBeginOverlap
  (params (OtherActor :type Actor%20Object%20Reference)))

(event EventTick
  (params (DeltaSeconds :type Float%20%28single-precision%29)))

(fn ConstructionScript)

(fn AddItem
  (params (Definition :type ST%20Item%20Instance%20Structure) (Count :type Integer))
  ;[0.15 0.09443 0.01816 0.5] Add Item to Inventory
  (LocalVariables|SetCountL Count)
  (LocalVariables|SetLen (Utilities|Array|Length (Variables|Default|GetItems)))
  (bind _output_get (LocalVariables|SetNewItemDef Definition))
  (Utilities|Struct|SetmembersinST_ItemInstance (LocalVariables|GetNewItemDef) Count)
  (LocalVariables|SetRemaining Count)
  (if (Utilities|IsValid (Utilities|Struct|BreakST_ItemInstance _output_get))
    (if (> (LocalVariables|GetLen) 0)
      (for (_array_element _array_index) (Variables|Default|GetItems)
        (LocalVariables|SetTempArrayElement _array_element)
        (if (and (== (Variables|/Game/Blueprins/Inventory/BP_ItemDefinition.BP_ItemDefinition_C|GetItemId (.definition (LocalVariables|GetNewItemDef))) (Variables|/Game/Blueprins/Inventory/BP_ItemDefinition.BP_ItemDefinition_C|GetItemId (Utilities|Struct|BreakST_ItemInstance (LocalVariables|GetTempArrayElement)))) (> (Variables|/Game/Blueprins/Inventory/BP_ItemDefinition.BP_ItemDefinition_C|GetMaxStack (.definition (LocalVariables|GetNewItemDef))) 1))
          (bind _output_get_2 (LocalVariables|SetRoom (- (Variables|/Game/Blueprins/Inventory/BP_ItemDefinition.BP_ItemDefinition_C|GetMaxStack (Utilities|Struct|BreakST_ItemInstance (LocalVariables|GetNewItemDef))) (Utilities|Struct|BreakST_ItemInstance (LocalVariables|GetTempArrayElement)))))
          (LocalVariables|SetbIsStack true)
          (LocalVariables|SetToAdd (Math|Integer|Min(Integer) _output_get_2 (LocalVariables|GetRemaining)))
          (Utilities|Struct|SetmembersinST_ItemInstance (LocalVariables|GetTempArrayElement) (+ (LocalVariables|GetToAdd) (Utilities|Struct|BreakST_ItemInstance (LocalVariables|GetTempArrayElement))))
          (LocalVariables|SetRemaining (- (LocalVariables|GetRemaining) (LocalVariables|GetToAdd)))
          (Utilities|Array|SetArrayElem (Variables|Default|GetItems) _array_index (LocalVariables|GetTempArrayElement))
          (if (<= (LocalVariables|GetRemaining) 0)
            (Default|CallOnItemsChanged)
            (return)
            (else
              (while (>= (LocalVariables|GetRemaining) 0)
                (bind _output_get_3 (LocalVariables|SetToPush (Math|Integer|Min(Integer) (LocalVariables|GetRemaining) (Variables|/Game/Blueprins/Inventory/BP_ItemDefinition.BP_ItemDefinition_C|GetMaxStack (Utilities|Struct|BreakST_ItemInstance (LocalVariables|GetNewItemDef))))))
                (Utilities|Array|Add (Variables|Default|GetItems) (Utilities|Struct|MakeST_ItemInstance (.Definition (Utilities|Struct|BreakST_ItemInstance (LocalVariables|GetTempArrayElement))) (LocalVariables|GetToPush) (Variables|/Game/Blueprins/Inventory/BP_ItemDefinition.BP_ItemDefinition_C|GetDurabilityMax (.Definition (Utilities|Struct|BreakST_ItemInstance (LocalVariables|GetTempArrayElement)))) (.InstanceId (Utilities|Struct|BreakST_ItemInstance (LocalVariables|GetTempArrayElement)))))
                (LocalVariables|SetRemaining (- (LocalVariables|GetRemaining) _output_get_3))
                (Default|CallOnItemsChanged)
                (return))))))
      (if (not (LocalVariables|GetbIsStack))
        (Utilities|Array|Add (Variables|Default|GetItems) (LocalVariables|GetNewItemDef))
        (Default|CallOnItemsChanged)
        (return))
      (else
        (bind _structout (Utilities|Struct|SetmembersinST_ItemInstance (LocalVariables|GetNewItemDef) (LocalVariables|GetCountL)))
        (Utilities|Array|Add (Variables|Default|GetItems) _structout)
        (Default|CallOnItemsChanged)
        (return)))
    (else
      (return))))

(fn Removeat
  (params (Index :type Integer) (Amount :type Integer))
  ;[0.15 0.1007 0.008952 0.5] Remove item from inventary
  (LocalVariables|SetAmontElem Amount)
  (bind _output_get (LocalVariables|SetIndexElem Index))
  (if (and (>= _output_get 0) (< (LocalVariables|GetIndexElem) (Utilities|Array|Length (Variables|Default|GetItems))))
    (bind _output_get_2 (LocalVariables|SetItem (Utilities|Array|Get(acopy) (Variables|Default|GetItems) (LocalVariables|GetIndexElem))))
    (Utilities|Struct|SetmembersinST_ItemInstance (LocalVariables|GetItem) (- (.Count (Utilities|Struct|BreakST_ItemInstance _output_get_2)) (LocalVariables|GetAmontElem)))
    (if (< (.Count (Utilities|Struct|BreakST_ItemInstance (LocalVariables|GetItem))) 0)
      (Utilities|Array|SetArrayElem (Variables|Default|GetItems) (LocalVariables|GetIndexElem) (LocalVariables|GetItem))
      (Default|CallOnItemsChanged)
      (else
        (Utilities|Array|RemoveIndex (Variables|Default|GetItems) (LocalVariables|GetIndexElem))
        (if (== (Variables|Default|GetActiveIndex) (LocalVariables|GetIndexElem))
          (CallFunction|SetActiveIndex -1)
          (Default|CallOnItemsChanged))))
    (else
      (return))))

(fn SetActiveIndex
  (params (NewIndex :type Integer))
  ;[0.04169 0.15 0.06705 0.5] Set Active Index DON'T FORGET TO ADD Equip \ UNEQUIP
  (Development|PrintString (Utilities|String|ToString(Integer) (Variables|Default|GetActiveIndex)))
  (LocalVariables|SetNewIndexL NewIndex)
  (LocalVariables|SetLen (+ (Utilities|Array|Length (Variables|Default|GetItems)) 1))
  (LocalVariables|SetWrapped (Math|Integer|%(Integer) (+ (Math|Integer|%(Integer) (LocalVariables|GetNewIndexL) (LocalVariables|GetLen)) (LocalVariables|GetLen)) (LocalVariables|GetLen)))
  (if (== (LocalVariables|GetWrapped) (Utilities|Array|Length (Variables|Default|GetItems)))
    (Variables|Default|SetActiveIndex -1)
    (CallFunction|Unequip)
    (Default|CallOnActiveItemChanged)
    (return)
    (else
      (Variables|Default|SetActiveIndex (LocalVariables|GetWrapped))
      (LocalVariables|SetDef (Utilities|Struct|BreakST_ItemInstance (Utilities|Array|Get(acopy) (Variables|Default|GetItems) (Variables|Default|GetActiveIndex))))
      (if (Utilities|IsValid (Utilities|Struct|BreakST_ItemInstance (Utilities|Array|Get(acopy) (Variables|Default|GetItems) (Variables|Default|GetActiveIndex))))
        (CallFunction|EquipfromDefinition (LocalVariables|GetDef))
        (else
          (CallFunction|Unequip))))))

(fn EquipfromDefinition
  (params (Definition :type BP%20Item%20Definition%20Object%20Reference))
  (bind _ownercharacter (Variables|Default|GetOwnerCharacter))
  ;[0.5732 0.1393 0.574 0.5] Equip Item
  (LocalVariables|SetDefenitionL Definition)
  (Utilities|FlowControl|Sequence
    (:then_0
      (if (Utilities|IsValid (Variables|Default|GetEquippedActor))
        (Actor|DestroyActor (Variables|Default|GetEquippedActor))
        (Variables|Default|SetEquippedActor 0)))
    (:then_1
      (Variables|Default|SetActiveBehaviorObject 0)
      (Variables|Default|SetActiveBehaviorObject 0))
    (:then_2
      (if (Utilities|IsValid (LocalVariables|GetDefenitionL))
        (if (Utilities|IsValidClass (Variables|/Game/Blueprins/Inventory/BP_ItemDefinition.BP_ItemDefinition_C|GetBehaviorActorClass (LocalVariables|GetDefenitionL)))
          (bind _returnvalue (Game|SpawnActorfromClass (Variables|/Game/Blueprins/Inventory/BP_ItemDefinition.BP_ItemDefinition_C|GetBehaviorActorClass (LocalVariables|GetDefenitionL)) (Transformation|GetActorTransform _ownercharacter) "AlwaysSpawn" "MultiplyWithRoot" 0 _ownercharacter))
          (bind _output_get (Variables|Default|SetEquippedActor _returnvalue))
          (Collision|SetActorEnableCollision _output_get false)
          (Transformation|AttachComponentToComponent _output_get (Variables|/Script/Engine.Character|GetMesh (Variables|Default|GetOwnerCharacter)) (Variables|/Game/Blueprins/Inventory/BP_ItemDefinition.BP_ItemDefinition_C|GetSocketName (LocalVariables|GetDefenitionL)) "SnapToTarget" "SnapToTarget" "SnapToTarget" true)
          (Transformation|SetActorRelativeTransform _output_get (Math|Transform|InvertTransform (Transformation|GetSocketTransform (Variables|/Script/Engine.Actor|GetRootComponent _output_get) (LocalVariables|GetSocketName) "RTS_Component")) false false)
          (elif (Utilities|IsValidClass (Variables|/Game/Blueprins/Inventory/BP_ItemDefinition.BP_ItemDefinition_C|GetBehaviorObjectClass (LocalVariables|GetDefenitionL)))
            (bind _returnvalue_2 (Game|ConstructObjectfromClass (Variables|/Game/Blueprins/Inventory/BP_ItemDefinition.BP_ItemDefinition_C|GetBehaviorObjectClass (LocalVariables|GetDefenitionL))))
            (Variables|Default|SetActiveBehaviorObject _returnvalue_2)
            (else
              (return))))
        (else
          (return))))
    (:then_3
      (Default|CallOnActiveItemChanged))))

(fn Unequip
  ;[0.06129 0.1156 0 0.5] Unequip
  (Variables|Default|SetActiveBehaviorObject 0)
  (bind _equippedactor (Variables|Default|GetEquippedActor)
    (:then
      (Actor|DestroyActor _equippedactor)
      (Variables|Default|SetEquippedActor 0))
    (:else)))

(fn UseActiveItem
  (params (User :type Character%20Object%20Reference))
  ;[0.9073 0.8948 0.01539 0.5] Use Active Item
  (LocalVariables|SetUserL User)
  (LocalVariables|SetLen (Utilities|Array|Length (Variables|Default|GetItems)))
  (LocalVariables|SetActiveObjects (and (Utilities|IsValid (Variables|Default|GetEquippedActor)) (Utilities|IsValid (Variables|Default|GetActiveBehaviorObject))))
  (if (and (>= (Variables|Default|GetActiveIndex) 0) (< (Variables|Default|GetActiveIndex) (LocalVariables|GetLen)))
    (bind _output_get (LocalVariables|SetInst (Utilities|Array|Get(acopy) (Variables|Default|GetItems) (Variables|Default|GetActiveIndex))))
    (bind _output_get_2 (LocalVariables|SetDef (Utilities|Struct|BreakST_ItemInstance _output_get)))
    (if (Utilities|IsValid _output_get_2)
      (if (LocalVariables|GetActiveObjects)
        (CallFunction|EquipfromDefinition (LocalVariables|GetDef))
        (if (Utilities|IsValid (Variables|Default|GetEquippedActor))
          (Utilities|FlowControl|Sequence
            (:then_0
              (if (Utilities|DoesObjectImplementInterface (Variables|Default|GetEquippedActor) "/Game/Blueprins/Inventory/IBP_InventoryItem.IBP_InventoryItem_C")
                (Class|IBPInventoryItem|Use(Message) (Variables|Default|GetEquippedActor) (LocalVariables|GetUserL))))
            (:then_1
              (if (Utilities|DoesObjectImplementInterface (Variables|Default|GetActiveBehaviorObject) "/Game/Blueprins/Inventory/IBP_InventoryItem.IBP_InventoryItem_C")
                (Class|IBPInventoryItem|Use(Message) (Variables|Default|GetActiveBehaviorObject) (LocalVariables|GetUserL)))))))
      (else
        (return)))
    (else
      (return))))

(fn ThrowActiveItem
  (params (User :type Character%20Object%20Reference) (Amount :type Integer))
  (bind _ownercharacter (Variables|Default|GetOwnerCharacter))
  ;[0.15 0.04902 0.02333 0.5] Throw Active Item
  (LocalVariables|SetUserL2 User)
  (LocalVariables|SetAmountL Amount)
  (LocalVariables|SetLen (Utilities|Array|Length (Variables|Default|GetItems)))
  (if (and (>= (Variables|Default|GetActiveIndex) 0) (< (Variables|Default|GetActiveIndex) (LocalVariables|GetLen)))
    (bind _output_get (LocalVariables|SetInst (Utilities|Array|Get(acopy) (Variables|Default|GetItems) (Variables|Default|GetActiveIndex))))
    (bind _output_get_2 (LocalVariables|SetDef (Utilities|Struct|BreakST_ItemInstance _output_get)))
    (if (Utilities|IsValid _output_get_2)
      (if (Variables|/Game/Blueprins/Inventory/BP_ItemDefinition.BP_ItemDefinition_C|GetbCanBeThrown (LocalVariables|GetDef))
        (bind _output_get_3 (LocalVariables|SetAmountClamped (Math|Integer|Clamp(Integer) (LocalVariables|GetAmountL) 1 (Utilities|Struct|BreakST_ItemInstance (LocalVariables|GetInst)))))
        (Utilities|FlowControl|Sequence
          (:then_0
            (if (<= _output_get_3 0)
              (return)
              (elif (and (Utilities|IsValid (Variables|Default|GetEquippedActor)) (Utilities|DoesObjectImplementInterface (Variables|Default|GetEquippedActor) "/Game/Blueprins/Inventory/IBP_InventoryItem.IBP_InventoryItem_C"))
                (Class|IBPInventoryItem|Throw(Message) (Variables|Default|GetEquippedActor) (LocalVariables|GetUserL2)))))
          (:then_1
            (if (and (Utilities|IsValid (Variables|Default|GetActiveBehaviorObject)) (Utilities|DoesObjectImplementInterface (Variables|Default|GetActiveBehaviorObject) "/Game/Blueprins/Inventory/IBP_InventoryItem.IBP_InventoryItem_C"))
              (Class|IBPInventoryItem|Throw(Message) (Variables|Default|GetActiveBehaviorObject) (LocalVariables|GetUserL2))))
          (:then_2
            (Utilities|FlowControl|Sequence
              (:then_1
                (bind _output_get_4 (LocalVariables|SetNearTransform (Math|Transform|MakeTransform (+ (Transformation|GetActorLocation _ownercharacter) (* (Transformation|GetActorForwardVector _ownercharacter) "0.000000,0.000000,50.000000")) (Transformation|GetActorRotation _ownercharacter))))
                (bind _returnvalue (Game|SpawnActorfromClass "/Game/Blueprins/01_Interaction/BP_WorldPickup.BP_WorldPickup_C" _output_get_4 "AlwaysSpawn" "MultiplyWithRoot" 0 (LocalVariables|GetInst) 0))
                (Default|ApplyThrow _returnvalue (Class|KismetMathLibrary|VectorNormalUnsafe (+ "0.000000,0.000000,0.300000" (Math|Vector|GetForwardVector (Variables|/Script/Engine.Character|GetCapsuleComponent (Variables|Default|GetOwnerCharacter))))) 4e+02)
                (CallFunction|Removeat (Variables|Default|GetActiveIndex) 1)
                (CallFunction|SetActiveIndex -1)))))
        (else
          (return)))
      (else
        (return)))
    (else
      (return))))