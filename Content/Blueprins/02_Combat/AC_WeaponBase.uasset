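; Base weapon Blueprint that lets an interacting player equip and throw a weapon, with an empty Attack event as a placeholder.
; OnEquip disables the supplied component's collision and snaps it to a named socket on the player's mesh.
; OnThrow, only while equipped, restores collision and applies a velocity-change impulse along the mesh's forward vector, without an explicit detach.
; IsInteactable always reports true.
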(event Custom|OnThrow
  (params (EquippableComponent :type Static%20Mesh%20Component%20Object%20Reference) (InteractingPlayer :type Character%20Object%20Reference))
  ;[0.1202 0.1397 0.15 0.5] On Throw Weapon
  (CallFunction|ThrowWeapon EquippableComponent (Variables|/Script/Engine.Character|GetMesh InteractingPlayer) 10))

(event Custom|OnEquip
  (params (EquippableComponent :type Static%20Mesh%20Component%20Object%20Reference) (InteractingPlayer :type Character%20Object%20Reference))
  ;[0.15 0.1118 0.002085 0.5] On Equip Weapon
  (bind _output_get (Variables|Default|SetEquippableComponent EquippableComponent))
  (Variables|Default|SetIsEquipped true)
  (CallFunction|Equipto _output_get (Variables|/Script/Engine.Character|GetMesh InteractingPlayer) (Variables|Default|GetEquipSocketName)))

(event EventBeginPlay)

(event EventTick
  (params (DeltaSeconds :type Float%20%28single-precision%29)))

(event EventAttack)

(fn Equipto
  (params (MeshToEquip :type Static%20Mesh%20Component%20Object%20Reference) (PerantMesh :type Skeletal%20Mesh%20Component%20Object%20Reference) (Socket :type Name))
  ;[0.15 0.1118 0.002085 0.5] On Equip Weapon
  (Collision|SetCollisionEnabled MeshToEquip "NoCollision")
  (Transformation|AttachComponentToComponent MeshToEquip PerantMesh Socket "SnapToTarget" "SnapToTarget" "SnapToTarget" true))

(fn IsInteactable
  (return true))

(fn ThrowWeapon
  (params (MeshToThrow :type Static%20Mesh%20Component%20Object%20Reference) (PlayerMesh :type Skeletal%20Mesh%20Component%20Object%20Reference) (ThrowForce :type Integer))
  ;[0.15 0.1239 0.1469 0.5] Throw Weapon
  (if (Variables|Default|GetIsEquipped)
    (Variables|Default|SetIsEquipped false)
    (Collision|SetCollisionEnabled MeshToThrow "QueryAndPhysics")
    (Physics|AddImpulse MeshToThrow (* ThrowForce (Math|Vector|GetForwardVector PlayerMesh)) "None" true)
    (else
      (return))))