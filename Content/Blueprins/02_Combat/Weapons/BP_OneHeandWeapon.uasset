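; BP_OneHeandWeapon is a one-handed weapon Blueprint that triggers an attack when used.
; Its Use event calls StartAttack on the user's BPCCombat component, leaving the attack logic to that component.
; The query functions return fixed values: it is interactable, cannot be thrown, and reports a zero count with an empty name and icon.
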(event EventUse
  (params (User :type BP%20Combat%20Character%20Base%20Object%20Reference))
  ;[0.7115 0.0467 0.03583 0.5] On Use Attack
  (Default|StartAttack (Variables|/Game/Blueprins/02_Combat/BP_CombatCharacterBase.BP_CombatCharacterBase_C|GetBPC_Combat User)))

(fn ConstructionScript)

(fn CanbeThrown
  (return false))

(fn GetCount
  (return 0))

(fn GetDisplayName
  (return ""))

(fn GetIcon
  (return ""))

(fn IsInteactable
  (return true))