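; BP_AxeWeapon is an axe weapon Blueprint that lets its user start a melee or combat attack.
; Its Use event forwards to the user's BPCCombat component by calling StartAttack, while its own Attack event is empty.
; The item query functions return placeholder values: it cannot be thrown, is not interactable, and has no count, name or icon.
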(event EventBeginPlay)

(event Collision|EventActorBeginOverlap
  (params (OtherActor :type Actor%20Object%20Reference)))

(event EventTick
  (params (DeltaSeconds :type Float%20%28single-precision%29)))

(event EventAttack)

(event EventUse
  (params (User :type BP%20Combat%20Character%20Base%20Object%20Reference))
  (Default|StartAttack (Variables|/Game/Blueprins/02_Combat/BP_CombatCharacterBase.BP_CombatCharacterBase_C|GetBPC_Combat User)))

(fn ConstructionScript)

(fn CanbeThrown
  (return false))

(fn GetCount
  (return 0))

(fn GetDisplayName
  (return ""))

(fn GetIcon
  (return ""))

(fn IsInteactable
  (return false))