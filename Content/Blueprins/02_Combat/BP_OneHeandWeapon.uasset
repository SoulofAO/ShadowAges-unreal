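; One-handed weapon Blueprint that makes its user perform a sword attack when used.
; The Use event calls StartAttack on the user with AM_SwordAttack, leaving the attack logic to the user.
; Item query functions report it as interactable and not throwable, while count, display name and icon return empty defaults.
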(event EventUse
  (params (User :type BP%20Combat%20Character%20Base%20Object%20Reference))
  ;[0.7115 0.0467 0.03583 0.5] On Use Attack
  (Default|StartAttack User "/Game/Blueprins/02_Combat/Anims/AM_SwordAttack.AM_SwordAttack"))

(fn ConstructionScript)

(fn CanbeThrown
  (return false))

(fn GetCount
  (return 0))

(fn GetDisplayName
  (return ""))

(fn GetIcon
  (return ""))

(fn IsInteactable
  (return true))