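; Base combat character Blueprint that ties together health, combat, melee and inventory, and exposes an attack-state check.
; It spawns and attaches an inventory actor, whose active-item changes set the current weapon and reinitialize the melee component with that weapon's damage.
; Incoming hits forward to the combat component, while a separate event binds to the health component's resolved-damage dispatcher.
; Death disables movement, limits collision to queries, plays a montage and destroys the actor afterward.
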(event Custom|OnDeathEvent
  ;[0.08248 0.076 0.15 0.5] On Death Event
  (bind _montagelength (CallFunction|OnDeath))
  (Utilities|FlowControl|Delay _montagelength)
  (Actor|DestroyActor))

(event Custom|ItemChanged
  (bind _returnvalue (Components|GetOwner))
  (bind _ac_meleecomponent (Variables|Default|GetAC_MeleeComponent))
  (bind _bpc_combat (Variables|Default|GetBPC_Combat))
  ;[0.7073 0.03282 0 0.5] Change on Active Current Weapon
  (bind _newparam (Default|GetEquipActor (Variables|Default|GetInventoryRef)))
  (bind _asbp_weapon_base (Utilities|Casting|CastToBP_WeaponBase _newparam)
    (:then
      (Default|SetCurrentWeapon _bpc_combat _asbp_weapon_base)
      (Default|Init _ac_meleecomponent _asbp_weapon_base _returnvalue (Math|Conversions|ToFloat(Integer) (Variables|/Game/Blueprins/02_Combat/BP_WeaponBase.BP_WeaponBase_C|GetDamage _asbp_weapon_base))))
    (:CastFailed
      (Default|SetCurrentWeapon _bpc_combat)
      (Default|Init _ac_meleecomponent 0 _returnvalue 0.0))))

(event Custom|OnTakeDamage
  ;[0.0375 0.15 0.1077 0.5] On Take Damage Event
  (EventDispatchers|BindEventtoOnDamageResolved (Variables|Default|GetAC_Health) (EventDispatchers|CreateEvent :!event TakeDamage)))

(event Collision|EventActorBeginOverlap
  (params (OtherActor :type Actor%20Object%20Reference)))

(event EventTick
  (params (DeltaSeconds :type Float%20%28single-precision%29)))

(fn ConstructionScript)

(fn CanAttack
  ;[0.7781 0.2058 0.04541 0.5] Return can attack state
  (return (not (Variables|Default|GetbIsAttacking))))

(fn BindInventoryEvents
  (bind _inventoryref (Variables|Default|GetInventoryRef))
  ;[0.7073 0.03282 0 0.5] Change on Active Current Weapon
  (if (Utilities|IsValid _inventoryref)
    (EventDispatchers|BindEventtoOnActiveItemChanged _inventoryref (EventDispatchers|CreateEvent :!event Custom|ItemChanged))))

(fn InitInventory
  ;[0.2452 0.1178 0.6656 0.5] Create inventory
  (bind _returnvalue (Game|SpawnActorfromClass "/Game/Blueprins/Inventory/BP_Inventory.BP_Inventory_C" (Transformation|GetActorTransform) "Undefined" "MultiplyWithRoot" 0 0))
  (Transformation|AttachComponentToComponent _returnvalue (Variables|Transformation|GetRootComponent) "None" "KeepRelative" "KeepRelative" "KeepRelative" true)
  (bind _output_get (Variables|Default|SetInventoryRef _returnvalue))
  (CallFunction|BindInventoryEvents)
  (return _output_get))

(fn OnDeath
  (bind _mesh (Variables|Character|GetMesh))
  (bind _returnvalue (Components|SkeletalMesh|GetAnimInstance _mesh))
  ;[0.7448 0.7259 0.7142 0.5] Death Logic
  (Pawn|Components|CharacterMovement|DisableMovement (Variables|Character|GetCharacterMovement))
  (Collision|SetCollisionEnabled (Variables|Collision|GetCapsuleComponent) "QueryOnly")
  (Animation|Montage|MontageStop _returnvalue 0.1 0)
  (bind _returnvalue_2 (Animation|Montage|MontagePlay _returnvalue "/Game/Blueprins/02_Combat/Anims/AM_Death.AM_Death" 1.0 "MontageLength" 0.0 true))
  (return _returnvalue_2))

(fn TakeDamage
  (params (ResponseHit :type E_HitResponse%20Enum :default "NewEnumerator0") (Damage :type Float%20%28double-precision%29) (Dot :type Float%20%28double-precision%29) (Cross :type Vector))
  (Default|TakeDamage (Variables|Default|GetBPC_Combat) ResponseHit Damage Dot Cross))