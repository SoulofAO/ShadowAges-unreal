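; Melee combat component for BP_CombatCharacterBase owners, handling combo attacks, blocking, hit reactions and timed combat mode.
; In combat mode, attacks play montages from the weapon's item data asset, queuing the next step during combo windows.
; A facing dot product decides whether blocks negate damage, and dot plus cross products pick directional hit montages.
; Offensive actions restart the combat timeout, and mode and block flags go directly to ABP_Unarmed through hard casts.
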(event Custom|RegisterOffensiveAction
  ;[0.04452 0.07636 0.15 0.5] Enable\disabled a Combat Mode
  (CallFunction|RegisterOffensive))

(event Custom|OnCombatTimerExpired
  ;[0.04452 0.07636 0.15 0.5] Enable\disabled a Combat Mode
  (CallFunction|ExpireCombat))

(event Custom|OpenComboWindow
  ;[0.324 0.03834 0.03199 0.5] Add Combo Events
  (Variables|Default|SetbInComboWindow true))

(event Custom|CloseComboWindow
  ;[0.324 0.03834 0.03199 0.5] Add Combo Events
  (Variables|Default|SetbInComboWindow false))

(event Custom|OnComboMontageEnded
  ;[0.324 0.03834 0.03199 0.5] Add Combo Events
  (CallFunction|ComboMontageEnded))

(event EventTick
  (params (DeltaSeconds :type Float%20%28single-precision%29)))

(fn SetCurrentWeapon
  (params (NewWeapon :type BP%20Weapon%20Base%20Object%20Reference))
  (Variables|Default|SetCurrentWeapon NewWeapon))

(fn StartAttack
  ;[0.5906 0.1356 0.5312 0.5] Start the Attack with property Montage
  (if (Variables|Default|GetbCanAttack)
    (if (Variables|Default|GetIsBlocking)
      (return)
      (elif (Utilities|IsValid (Variables|Default|GetCurrentWeapon))
        (if (Variables|Default|GetIsInCompat)
          (bind _len (Default|GetComboMontageCount (Variables|Default|GetCurrentWeapon)))
          (bind _output_get (Variables|Default|SetCount _len))
          (if (> _output_get 0)
            (if (Variables|Default|GetbIsAttacking)
              (bind _output_get_2 (LocalVariables|SetNextIndex%20 (+ (Variables|Default|GetCurrentComboIndex) 1)))
              (if (and (Variables|Default|GetbInComboWindow) (< _output_get_2 (Variables|Default|GetCount)))
                (Variables|Default|SetbComboQueued true))
              (else
                (Variables|Default|SetbIsAttacking true)
                (CallFunction|PlayComboStep)))
            (else
              (return)))
          (else
            (CallFunction|EndAttack)
            (return)))
        (else
          (return))))
    (else
      (return))))

(fn PlayComboStep
  ;[0.03168 0.0164 0.15 0.5] Player Combo Montage
  (CallFunction|StopBlock)
  (bind _asda_item_definition (Utilities|Casting|CastToDA_ItemDefinition (Utilities|Struct|BreakST_ItemInstance (Variables|/Game/Blueprins/02_Combat/Weapons/BP_WeaponBase.BP_WeaponBase_C|GetItem (Variables|Default|GetCurrentWeapon))))
    (:then
      (if (Utilities|IsValid (Variables|Default|GetCurrentWeapon))
        (if (Utilities|IsValid (Utilities|Array|Get(acopy) (Variables|/Game/Blueprins/Inventory/DA_ItemDefinition.DA_ItemDefinition_C|GetMontages _asda_item_definition) (Variables|Default|GetCurrentComboIndex)))
          (bind _asbp_combat_character_base (Utilities|Casting|CastToBP_CombatCharacterBase (Components|GetOwner))
            (:then
              (Animation|Montage|MontagePlay (Components|SkeletalMesh|GetAnimInstance (Variables|/Script/Engine.Character|GetMesh _asbp_combat_character_base)) (Utilities|Array|Get(acopy) (Variables|/Game/Blueprins/Inventory/DA_ItemDefinition.DA_ItemDefinition_C|GetMontages _asda_item_definition) (Variables|Default|GetCurrentComboIndex)) 1.0 "MontageLength" 0.0 false))
            (:CastFailed
              (return)))
          (else
            (return)))))
    (:CastFailed
      (return))))

(fn EndAttack
  ;[0.01917 0.15 0.01357 0.5] End Attack And Full Reset Attack State + calling dispatecher
  (CallFunction|ResetComboState)
  (Default|CallOnAttackFinished)
  (Default|CallOnAttackFinished))

(fn ResetComboState
  ;[0.03763 0.15 0.03614 0.833] ResetStates
  (Variables|Default|SetbIsAttacking false)
  (Variables|Default|SetbInComboWindow false)
  (Variables|Default|SetbComboQueued false)
  (Variables|Default|SetCurrentComboIndex 0))

(fn ComboMontageEnded
  ;[0.8406 0.7455 0.06973 0.5] End Combo window
  (bind _output_get (LocalVariables|SetNextIndex (+ (Variables|Default|GetCurrentComboIndex) 1)))
  (if (and (<= (LocalVariables|GetNextIndex) (Variables|Default|GetCount)) (Variables|Default|GetbComboQueued))
    (Variables|Default|SetCurrentComboIndex _output_get)
    (CallFunction|PlayComboStep)
    (else
      (Variables|Default|SetbInComboWindow false)
      (Variables|Default|SetbComboQueued false)
      (Variables|Default|SetCurrentComboIndex 0)
      (Default|CallOnAttackFinished))))

(fn RegisterOffensive
  ;[0.3413 0.5276 1 0.5] Enable a combat mode TO DO ПЕРЕДЕЛАТЬ ТО ЧТО Я КАСЧУ НА ОПРЕДЕЛЕННЫЙ АНИМАТОР НА ЧТО-ТО НОРМАЛЬНОЕ!!!!
  (Variables|Default|SetIsInCompat true)
  (bind _asbp_combat_character_base (Utilities|Casting|CastToBP_CombatCharacterBase (Components|GetOwner)))
  (bind _asabp_unarmed (Utilities|Casting|CastToABP_Unarmed (Components|SkeletalMesh|GetAnimInstance (Variables|/Script/Engine.Character|GetMesh _asbp_combat_character_base))))
  (Default|CombatMode _asabp_unarmed true)
  (Utilities|Time|ClearandInvalidateTimerbyHandle (Variables|Default|GetCombatTimerHandle))
  (bind _returnvalue (Utilities|Time|SetTimerbyFunctionName 0 (Variables|Default|GetFunctionName) (Variables|Default|GetCombatTimeout)))
  (Variables|Default|SetCombatTimerHandle _returnvalue))

(fn ExpireCombat
  ;[0.06759 0.03356 0.15 0.5] Disable a Combat Mod TO DO ПЕРЕДЕЛАТЬ ТО ЧТО Я КАСЧУ НА ОПРЕДЕЛЕННЫЙ АНИМАТОР НА ЧТО-ТО НОРМАЛЬНОЕ!!!!
  (Variables|Default|SetIsInCompat false)
  (bind _asbp_combat_character_base (Utilities|Casting|CastToBP_CombatCharacterBase (Components|GetOwner)))
  (Utilities|Time|ClearandInvalidateTimerbyHandle (Variables|Default|GetCombatTimerHandle))
  (bind _asabp_unarmed (Utilities|Casting|CastToABP_Unarmed (Components|SkeletalMesh|GetAnimInstance (Variables|/Script/Engine.Character|GetMesh _asbp_combat_character_base))))
  (Default|CombatMode _asabp_unarmed (Variables|Default|GetIsInCompat)))

(fn StartBlock
  ;[0.03573 0.15 0.07292 0.5] Start block TO DO ПЕРЕДЕЛАТЬ ТО ЧТО Я КАСЧУ НА ОПРЕДЕЛЕННЫЙ АНИМАТОР НА ЧТО-ТО НОРМАЛЬНОЕ!!!!
  (CallFunction|RegisterOffensive)
  (bind _return (CallFunction|CasttoAnimBP))
  (Default|BlockMode _return true)
  (Variables|Default|SetIsBlocking true)
  (bind _asbp_combat_character_base (Utilities|Casting|CastToBP_CombatCharacterBase (Components|GetOwner))
    (:then
      (bind _asda_item_definition (Utilities|Casting|CastToDA_ItemDefinition (Utilities|Struct|BreakST_ItemInstance (Variables|/Game/Blueprins/02_Combat/Weapons/BP_WeaponBase.BP_WeaponBase_C|GetItem (Variables|Default|GetCurrentWeapon))))
        (:then
          (Animation|Montage|MontagePlay (Components|SkeletalMesh|GetAnimInstance (Variables|/Script/Engine.Character|GetMesh _asbp_combat_character_base)) (Variables|/Game/Blueprins/Inventory/DA_ItemDefinition.DA_ItemDefinition_C|GetBlockMontage _asda_item_definition) 1.0 "MontageLength" 0.0 false)
          (Class|AnimInstance|MontageSetNextSection (Components|SkeletalMesh|GetAnimInstance (Variables|/Script/Engine.Character|GetMesh _asbp_combat_character_base)) "Enter" "Loop" (Variables|/Game/Blueprins/Inventory/DA_ItemDefinition.DA_ItemDefinition_C|GetBlockMontage _asda_item_definition)))
        (:CastFailed
          (return))))
    (:CastFailed
      (return))))

(fn StopBlock
  ;[0.0454 0.02953 0.15 0.5] Stop block TO DO ПЕРЕДЕЛАТЬ ТО ЧТО Я КАСЧУ НА ОПРЕДЕЛЕННЫЙ АНИМАТОР НА ЧТО-ТО НОРМАЛЬНОЕ!!!!
  (bind _return (CallFunction|CasttoAnimBP))
  (Default|BlockMode _return false)
  (Variables|Default|SetIsBlocking false)
  (bind _asbp_combat_character_base (Utilities|Casting|CastToBP_CombatCharacterBase (Components|GetOwner))
    (:then
      (bind _asda_item_definition (Utilities|Casting|CastToDA_ItemDefinition (Utilities|Struct|BreakST_ItemInstance (Variables|/Game/Blueprins/02_Combat/Weapons/BP_WeaponBase.BP_WeaponBase_C|GetItem (Variables|Default|GetCurrentWeapon))))
        (:then
          (Ability|Animation|MontageJumptoSection (Components|SkeletalMesh|GetAnimInstance (Variables|/Script/Engine.Character|GetMesh _asbp_combat_character_base)) "End" (Variables|/Game/Blueprins/Inventory/DA_ItemDefinition.DA_ItemDefinition_C|GetBlockMontage _asda_item_definition)))
        (:CastFailed
          (return))))
    (:CastFailed
      (return))))

(fn ComputeDamageResponse
  (params (Damage :type Float%20%28double-precision%29) (DamageCauser :type Actor%20Object%20Reference))
  ;[0.03038 0.09858 0.15 0.5] Block Attack Logic
  (LocalVariables|SetIncomingDamage Damage)
  (LocalVariables|SetDamageActor DamageCauser)
  (bind (_dot _cross) (CallFunction|CalculateCrossandDot (LocalVariables|GetDamageActor)))
  (LocalVariables|SetDot _dot)
  (LocalVariables|SetCross _cross)
  (if (Variables|Default|GetIsBlocking)
    (if (Utilities|IsValid (LocalVariables|GetDamageActor))
      (if (>= (LocalVariables|GetDot) (Variables|Default|GetBlockDotThreshold))
        (return "NewEnumerator1" 0.0 (LocalVariables|GetDot) (LocalVariables|GetCross))
        (else
          (return "NewEnumerator0" (LocalVariables|GetIncomingDamage) (LocalVariables|GetDot) (LocalVariables|GetCross))))
      (else
        (return "NewEnumerator0" (LocalVariables|GetIncomingDamage) (LocalVariables|GetDot) (LocalVariables|GetCross))))
    (else
      (return "NewEnumerator0" (LocalVariables|GetIncomingDamage) (LocalVariables|GetDot) (LocalVariables|GetCross)))))

(fn CasttoAnimBP
  ;[0.06639 0.04973 0.15 0.5] Return anim bp ИСПРАВИТЬ НА НОРМ
  (bind _asbp_combat_character_base (Utilities|Casting|CastToBP_CombatCharacterBase (Components|GetOwner)))
  (bind _asabp_unarmed (Utilities|Casting|CastToABP_Unarmed (Components|SkeletalMesh|GetAnimInstance (Variables|/Script/Engine.Character|GetMesh _asbp_combat_character_base))))
  (return _asabp_unarmed))

(fn ReciveHit
  (params (DamageType :type E_HitResponse%20Enum :default "NewEnumerator0") (Damage :type Float%20%28double-precision%29) (Dot :type Float%20%28double-precision%29) (Cross :type Vector))
  ;[0.1387 0.1853 0.7573 0.5] Play Damage Montage by Event
  (CallFunction|ResetComboState)
  (LocalVariables|SetDotL Dot)
  (LocalVariables|SetCrossL Cross)
  (bind _asbp_combat_character_base (Utilities|Casting|CastToBP_CombatCharacterBase (Components|GetOwner)))
  (switch Utilities|FlowControl|Switch|SwitchonE_HitResponse DamageType
    (:NewEnumerator0
      (Variables|Default|SetbCanAttack false)
      (Animation|Montage|MontageStop (Components|SkeletalMesh|GetAnimInstance (Variables|/Script/Engine.Character|GetMesh _asbp_combat_character_base)) 0.2 0)
      (bind _montage (CallFunction|GetHitMontage (LocalVariables|GetDotL) (LocalVariables|GetCrossL)))
      (bind _returnvalue (Animation|Montage|MontagePlay (Components|SkeletalMesh|GetAnimInstance (Variables|/Script/Engine.Character|GetMesh _asbp_combat_character_base)) _montage 1.0 "MontageLength" 0.0 true))
      (return _returnvalue))
    (:NewEnumerator1
      (return 0.0))))

(fn CalculateCrossandDot
  (params (DamageCauser :type Actor%20Object%20Reference))
  (bind _returnvalue (Components|GetOwner))
  ;[0.05578 0.15 0.05322 0.5] Calculate Dot and cross of damage couser
  (LocalVariables|SetDamageActor DamageCauser)
  (if (Utilities|IsValid (LocalVariables|GetDamageActor))
    (LocalVariables|SetAttackerLocation (Transformation|GetActorLocation (LocalVariables|GetDamageActor)))
    (LocalVariables|SetOwnerLocation (Transformation|GetActorLocation _returnvalue))
    (LocalVariables|SetOwnerForward (Transformation|GetActorForwardVector _returnvalue))
    (bind _output_get (LocalVariables|SetDirToAttacker (- (LocalVariables|GetAttackerLocation) (LocalVariables|GetOwnerLocation))))
    (bind _output_get_2 (LocalVariables|SetDirToAttackerNormalized (Math|Vector|Normalize _output_get)))
    (return (Math|Vector|DotProduct (LocalVariables|GetOwnerForward) _output_get_2) (Math|Vector|CrossProduct (LocalVariables|GetOwnerForward) (LocalVariables|GetDirToAttackerNormalized)))))

(fn GetHitMontage
  (params (Dot :type Float%20%28double-precision%29) (Cross :type Vector))
  ;[0.2209 0.3592 0.674 0.5] Return Hit Montage
  (LocalVariables|SetDotL Dot)
  (LocalVariables|SetCrossL Cross)
  (if (> (LocalVariables|GetDotL) 0.5)
    (return (.Value (Utilities|Map|Find (Variables|Default|GetDamageAnim) "NewEnumerator2")))
    (elif (< (LocalVariables|GetDotL) -0.5)
      (return (.Value (Utilities|Map|Find (Variables|Default|GetDamageAnim) "NewEnumerator3")))
      (elif (>= (.z (LocalVariables|GetCrossL)) 0.0)
        (return (.Value (Utilities|Map|Find (Variables|Default|GetDamageAnim) "NewEnumerator0")))
        (else
          (return (.Value (Utilities|Map|Find (Variables|Default|GetDamageAnim) "NewEnumerator1"))))))))