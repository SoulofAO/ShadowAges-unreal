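; Actor component for melee weapons that detects hits during a timed hit window and applies damage.
; Starting the window records weapon socket locations and starts a looping timer for tracing.
; PerformTrace sphere-sweeps from previous to current socket positions, reading sockets from WeaponMesh or falling back to the weapon's static mesh.
; It skips the instigator and already-hit actors, and applies damage only with authority.
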(event EventBeginPlay)

(event EventTick
  (params (DeltaSeconds :type Float%20%28single-precision%29)))

(fn Init
  (params (OwnerWeapon :type Actor%20Object%20Reference) (Instigator :type Actor%20Object%20Reference))
  ;[0.1707 0.2815 0.7156 0.5] Init function
  (Variables|Default|SetOwnerWeapon OwnerWeapon)
  (Variables|Default|SetInstigatorActor Instigator)
  (Utilities|Array|Clear (Variables|Default|GetPrevSockets))
  (Utilities|Set|Clear (Variables|Default|GetAlreadyHit)))

(fn StartHitWindow
  ;[0.1448 0.8115 0.1517 0.5] StartHitWindow
  (Variables|Default|SetbHitWindow true)
  (Utilities|Set|Clear (Variables|Default|GetAlreadyHit))
  (for _array_element (Variables|Default|GetSocketNames)
    (Utilities|IsValid (Variables|Default|GetWeaponMesh)
      (:Is%20Valid
        (Utilities|Array|Add (Variables|Default|GetPrevSockets) (Transformation|GetSocketLocation (Variables|Default|GetWeaponMesh) _array_element)))
      (:Is%20Not%20Valid
        (Utilities|Array|Add (Variables|Default|GetPrevSockets) (Transformation|GetSocketLocation (Actor|GetComponentbyClass (Variables|Default|GetOwnerWeapon) "/Script/Engine.StaticMeshComponent") _array_element)))))
  (Utilities|Time|SetTimerbyEvent (EventDispatchers|CreateEvent :!event PerformTrace) (Variables|Default|GetTraceInterval) true))

(fn EndHitWindow
  ;[0.9073 0.293 0.004725 0.5] End Hit Window
  (Variables|Default|SetbHitWindow false)
  (Utilities|Time|ClearTimerbyFunctionName 0 (LocalVariables|GetFunctionName)))

(fn GetOwnerMesh
  (Utilities|IsValid (Variables|Default|GetWeaponMesh)))

(fn PerformTrace
  ;[0.1935 0.1651 0.7198 0.5] Calulate Damage Zone By Sockets and Apply Damage
  (if (Variables|Default|GetbHitWindow)
    (Utilities|Array|Clear (Variables|Default|GetCurrentSockets))
    (for _array_element (Variables|Default|GetSocketNames)
      (if (Utilities|IsValid (Variables|Default|GetWeaponMesh))
        (Utilities|Array|Add (Variables|Default|GetCurrentSockets) (Transformation|GetSocketLocation (Variables|Default|GetWeaponMesh) _array_element))
        (else
          (Utilities|Array|Add (Variables|Default|GetCurrentSockets) (Transformation|GetSocketLocation (Actor|GetComponentbyClass (Variables|Default|GetOwnerWeapon) "/Script/Engine.StaticMeshComponent") _array_element)))))
    (Collision|MultiSphereTraceByChannel "0, 0, 0" "0, 0, 0" 0.0 "TraceTypeQuery1" false 0 (select (Variables|Default|GetDebugDraw) "ForDuration" "None"))
    (for (_array_element_2 _array_index) (Variables|Default|GetPrevSockets)
      (LocalVariables|SetTempIndex _array_index)
      (LocalVariables|SetPrev _array_element_2)
      (LocalVariables|SetCur (Utilities|Array|Get(acopy) (Variables|Default|GetCurrentSockets) (LocalVariables|GetTempIndex)))
      (bind _outhits (Collision|MultiSphereTraceByChannel (LocalVariables|GetPrev) (LocalVariables|GetCur) (Variables|Default|GetTraceRadius) (Variables|Default|GetTraceChannel) false 0 (LocalVariables|GetDrawMode)))
      (bind _output_get (LocalVariables|SetHitResults _outhits))
      (for _array_element_3 _output_get
        (bind _output_get_2 (LocalVariables|SetHitActor (.HitActor (Collision|BreakHitResult _array_element_3))))
        (if (Utilities|IsValid _output_get_2)
          (if (not (== (LocalVariables|GetHitActor) (Variables|Default|GetInstigatorActor)))
            (if (not (Utilities|Set|Contains (Variables|Default|GetAlreadyHit) (LocalVariables|GetHitActor)))
              (Networking|SwitchHasAuthority
                (:Authority
                  (bind _aspawn (Utilities|Casting|CastToPawn (Variables|Default|GetInstigatorActor)))
                  (Game|Damage|ApplyDamage (LocalVariables|GetHitActor) (Variables|Default|GetDamage) (Pawn|GetController _aspawn) (Variables|Default|GetOwnerWeapon))
                  (Utilities|Set|Add (Variables|Default|GetAlreadyHit) (LocalVariables|GetHitActor))))))))
      (Variables|Default|SetPrevSockets (Variables|Default|GetCurrentSockets))
      (return))
    (else
      (return))))