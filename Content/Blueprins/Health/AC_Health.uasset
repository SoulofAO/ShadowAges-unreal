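; Health component that tracks an actor's health, applying damage, healing capped at MaxHealth, and death.
; On BeginPlay it fills Health and binds to the owner's OnTakeAnyDamage event.
; Incoming damage passes through BPC_Combat's ComputeDamageResponse when the damaged actor has that component, then reduces Health.
; Damage exceeding remaining Health zeroes it and calls OnDeath on a BP_CombatCharacterBase owner; exactly zero does not.
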(event EventBeginPlay
  ;[0.15 0.01215 0.01961 0.5] Init Damage Consume
  (Utilities|FlowControl|Sequence
    (:then_0
      (Variables|Default|SetHealth (Variables|Default|GetMaxHealth)))
    (:then_1
      (EventDispatchers|BindEventtoOnTakeAnyDamage (Components|GetOwner) (EventDispatchers|CreateEvent :!event GetDamagedEvent)))))

(fn GetDamaged
  (params (Damage :type Float%20%28double-precision%29))
  ;[0.15 0.007202 0 0.5] On Damage  function
  (LocalVariables|SetdamagedHealth (- (Variables|Default|GetHealth) Damage))
  (if (>= (LocalVariables|GetdamagedHealth) 0.0)
    (Variables|Default|SetHealth (LocalVariables|GetdamagedHealth))
    (else
      (Variables|Default|SetHealth 0.0)
      (bind _asbp_combat_character_base (Utilities|Casting|CastToBP_CombatCharacterBase (Components|GetOwner)))
      (Default|OnDeath _asbp_combat_character_base))))

(fn GetDamagedEvent
  (params (DamagedActor :type Actor%20Object%20Reference) (Damage :type Float%20%28single-precision%29) (DamageType :type Damage%20Type%20Object%20Reference) (InstigatedBy :type Controller%20Object%20Reference) (DamageCauser :type Actor%20Object%20Reference))
  (bind _returnvalue (Actor|GetComponentbyClass DamagedActor "/Game/Blueprins/02_Combat/BPC_Combat.BPC_Combat_C"))
  ;[0.15 0.007202 0 0.5] On Damage Event Binding
  (if (Utilities|IsValid _returnvalue)
    (bind _finaldamage (Default|ComputeDamageResponse _returnvalue Damage DamageCauser))
    (LocalVariables|SetLocalDamage _finaldamage)
    (else
      (LocalVariables|SetLocalDamage Damage)))
  (CallFunction|GetDamaged (LocalVariables|GetLocalDamage)))

(fn GetHeald
  (params (Heal :type Float%20%28double-precision%29))
  ;[0.01556 0.15 0.05013 0.5] Get Heald Function
  (LocalVariables|SetSummedHealth (+ Heal (Variables|Default|GetHealth)))
  (if (> (LocalVariables|GetSummedHealth) (Variables|Default|GetMaxHealth))
    (Variables|Default|SetHealth (Variables|Default|GetMaxHealth))
    (else
      (Variables|Default|SetHealth (LocalVariables|GetSummedHealth)))))