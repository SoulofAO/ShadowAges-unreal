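; BP_HealthBox is a healing volume that periodically restores health to an actor overlapping its HealBox.
; Begin overlap stores the actor and starts a looping one-second timer, which calls GetHeald on the actor's AC_Health component with HealValue.
; Any end overlap clears the stored timer.
; Only one actor and timer handle are stored, so a new overlap overwrites both, and no actor filter or validity check exists.
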(event OnComponentBeginOverlap(HealBox)
  (params (OverlappedComponent :type Primitive%20Component%20Object%20Reference) (OtherActor :type Actor%20Object%20Reference) (OtherComp :type Primitive%20Component%20Object%20Reference) (OtherBodyIndex :type Integer) (bFromSweep :type Boolean) (SweepResult :type Hit%20Result%20Structure%20%28by%20ref%29))
  ;[0.01556 0.15 0.05013 0.5] On Heal per second on box overlap
  (Variables|Default|SetOtherActorRef OtherActor)
  (bind _returnvalue (Utilities|Time|SetTimerbyEvent (delegate Custom|Heal) 1.0 true))
  (Variables|Default|SetTimerReference _returnvalue))

(event OnComponentEndOverlap(HealBox)
  (params (OverlappedComponent :type Primitive%20Component%20Object%20Reference) (OtherActor :type Actor%20Object%20Reference) (OtherComp :type Primitive%20Component%20Object%20Reference) (OtherBodyIndex :type Integer))
  ;[0.133 0.15 0.1219 0.5] Off Heal per second on box overlap
  (Utilities|Time|ClearandInvalidateTimerbyHandle (Variables|Default|GetTimerReference)))

(event Custom|Heal
  ;[0.01556 0.15 0.05013 0.5] On Heal per second on box overlap
  (Default|GetHeald (Actor|GetComponentbyClass (Variables|Default|GetOtherActorRef) "/Game/Blueprins/Health/AC_Health.AC_Health_C") (Variables|Default|GetHealValue)))

(fn ConstructionScript)