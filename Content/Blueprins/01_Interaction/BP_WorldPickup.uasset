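; World item pickup that displays its item definition's skeletal mesh, or static mesh as fallback, chosen on BeginPlay or through InitPickup.
; InitPickup also stores count and durability and applies world scale.
; Interacting adds the item to the combat character's inventory, then OnEquip activates the last slot and destroys the pickup for third-person characters.
; Throws apply a physics impulse to the static mesh; FrozePhysics is unwired.
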(event Custom|ApplyThrow
  (params (Direction :type Vector) (Strength :type Float%20%28double-precision%29))
  (bind _staticmeshcomponent (Variables|Default|GetStaticMeshComponent))
  ;[0.5781 0 0.02089 0.5] Throw Event
  (Physics|SetSimulatePhysics _staticmeshcomponent true)
  (Physics|AddImpulse _staticmeshcomponent (* Direction Strength) "None" true))

(event EventBeginPlay
  ;[0.5781 0 0.02089 0.5] Begin Play
  (CallFunction|Init))

(event Collision|EventActorBeginOverlap
  (params (OtherActor :type Actor%20Object%20Reference)))

(event EventTick
  (params (DeltaSeconds :type Float%20%28single-precision%29)))

(event EventOnInteract
  (params (InteractingPlayer :type Character%20Object%20Reference))
  ;[0.3367 0.1684 1 0.5] On Equip Interact
  (bind _asbp_combat_character_base (Utilities|Casting|CastToBP_CombatCharacterBase InteractingPlayer))
  (Default|AddItem (Variables|/Game/Blueprins/02_Combat/BP_CombatCharacterBase.BP_CombatCharacterBase_C|GetInventoryRef _asbp_combat_character_base) (Variables|Default|GetDefinition) (Variables|Default|GetCount))
  (CallFunction|OnEquip InteractingPlayer))

(fn ConstructionScript)

(fn OnEquip
  (params (InteractingPlayer :type Character%20Object%20Reference))
  ;[0.3367 0.1684 1 0.5] On Equip Interact
  (bind _asbp_third_person_character (Utilities|Casting|CastToBP_ThirdPersonCharacter InteractingPlayer))
  (LocalVariables|SetInventory (Variables|/Game/Blueprins/02_Combat/BP_CombatCharacterBase.BP_CombatCharacterBase_C|GetInventoryRef _asbp_third_person_character))
  (if (Utilities|IsValid (LocalVariables|GetInventory))
    (bind _output_get (LocalVariables|SetLen2 (Utilities|Array|Length (Variables|/Game/Blueprins/Inventory/BP_Inventory.BP_Inventory_C|GetItems (LocalVariables|GetInventory)))))
    (Utilities|FlowControl|Sequence
      (:then_0
        (if (> _output_get 0)
          (Default|SetActiveIndex (LocalVariables|GetInventory) (- (LocalVariables|GetLen2) 1))))
      (:then_1
        (Actor|DestroyActor)))
    (else
      (return))))

(fn InitPickup
  (params (Definition :type BP%20Item%20Definition%20Object%20Reference) (Count :type Integer) (Durability :type Integer))
  (bind _skeletalmesh (Variables|Default|GetSkeletalMesh))
  (bind _staticmeshcomponent (Variables|Default|GetStaticMeshComponent))
  (bind _definition (Utilities|Struct|BreakST_ItemInstance (Variables|Default|GetDefinition)))
  (bind _definition_2 (Utilities|Struct|BreakST_ItemInstance (Variables|Default|GetDefinition)))
  (bind _worldscale (Variables|/Game/Blueprins/Inventory/BP_ItemDefinition.BP_ItemDefinition_C|GetWorldScale _definition_2))
  (bind _skeletalmesh_2 (Variables|/Game/Blueprins/Inventory/BP_ItemDefinition.BP_ItemDefinition_C|GetSkeletalMesh _definition))
  ;[0 0.6198 0.2985 0.5] Init function
  (Variables|Default|SetCount Count)
  (Variables|Default|SetDurability Durability)
  (Utilities|Struct|SetmembersinST_ItemInstance (Variables|Default|GetDefinition) Definition Count Durability)
  (Utilities|FlowControl|Sequence
    (:then_0
      (if (Utilities|IsValid _skeletalmesh_2)
        (Components|SkeletalMesh|SetSkeletalMeshAsset _skeletalmesh _skeletalmesh_2)
        (Rendering|SetVisibility _skeletalmesh true true)
        (Rendering|SetVisibility (Variables|Default|GetStaticMeshComponent) false false)
        (Transformation|SetWorldScale3D _skeletalmesh _worldscale)
        (else
          (Components|StaticMesh|SetStaticMesh _staticmeshcomponent (Variables|/Game/Blueprins/Inventory/BP_ItemDefinition.BP_ItemDefinition_C|GetStaticMesh _definition))
          (Rendering|SetVisibility _staticmeshcomponent true true)
          (Rendering|SetVisibility (Variables|Default|GetSkeletalMesh) false true)
          (Transformation|SetWorldScale3D (Variables|Default|GetStaticMeshComponent) _worldscale))))))

(fn Init
  (bind _staticmeshcomponent (Variables|Default|GetStaticMeshComponent))
  (bind _skeletalmesh (Variables|Default|GetSkeletalMesh))
  (bind _definition (Variables|Default|GetDefinition))
  (bind _definition_2 (Utilities|Struct|BreakST_ItemInstance _definition))
  ;[0.5781 0 0.02089 0.5] Begin Play
  (if (Utilities|IsValid (Variables|/Game/Blueprins/Inventory/BP_ItemDefinition.BP_ItemDefinition_C|GetSkeletalMesh (Utilities|Struct|BreakST_ItemInstance (Variables|Default|GetDefinition))))
    (Components|SkeletalMesh|SetSkeletalMeshAsset _skeletalmesh (Variables|/Game/Blueprins/Inventory/BP_ItemDefinition.BP_ItemDefinition_C|GetSkeletalMesh _definition_2))
    (Rendering|SetVisibility _skeletalmesh true true)
    (Rendering|SetVisibility (Variables|Default|GetStaticMeshComponent) false true)
    (else
      (Components|StaticMesh|SetStaticMesh _staticmeshcomponent (Variables|/Game/Blueprins/Inventory/BP_ItemDefinition.BP_ItemDefinition_C|GetStaticMesh _definition_2))
      (Rendering|SetVisibility _staticmeshcomponent true true)
      (Rendering|SetVisibility (Variables|Default|GetSkeletalMesh) false true))))

(fn FrozePhysics)

(fn IsInteactable
  (return true))